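; Actor component that tracks health and handles damage, healing and death notification.
; Health starts at MaxHealth on BeginPlay, and every change goes through UpdateHealth, which broadcasts the new value.
; TakeDamage and Heal also fire their own dispatchers, with OnDeath called whenever damage leaves health at or below zero.
; Healing is clamped between zero and MaxHealth, while damage is unclamped.
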(event EventBeginPlay
  (CallFunction|UpdateHealth (Variables|Default|GetmaxHealth)))

(fn TakeDamage
  (params (damage :type Float%20%28double-precision%29))
  (CallFunction|UpdateHealth (- (Variables|Default|GetHealth) damage))
  (Default|CallOnTakeDamage)
  (if (<= (Variables|Default|GetHealth) 0.0)
    (Default|CallOnDeath)))

(fn Heal
  (params (value :type Float%20%28double-precision%29))
  (CallFunction|UpdateHealth (Math|Float|Clamp(Float) (+ (Variables|Default|GetHealth) value) 0.0 (Variables|Default|GetmaxHealth)))
  (Default|CallOnHeal))

(fn UpdateHealth
  (params (newHealthValue :type Float%20%28double-precision%29))
  (bind _output_get (Variables|Default|SetHealth newHealthValue))
  (Default|CallOnHealthUpdate _output_get))